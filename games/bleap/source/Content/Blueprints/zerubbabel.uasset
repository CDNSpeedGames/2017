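; Player Character Blueprint that handles basic jump, look and movement input.
; Jump press and release start and stop jumping, while movement axes add input along right and forward vectors built from control yaw alone.
; The look handlers are crossed relative to their names: LookUpDown drives controller yaw and TurnLeftRight drives pitch.
; The construction script is empty.
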(event `InputAction|Jump`
  (params (Key :type "Key Structure"))
  ;[1 1 1] Player Jump
  (:`Pressed`
    (`self.Jump`))
  (:`Released`
    (`self.StopJumping`)))

(event `InputAxis|LookUpDown`
  (params (AxisValue :type "Float (single-precision)"))
  ;[1 1 1] Look Up and Down
  (`self.AddControllerYawInput` AxisValue))

(event `InputAxis|TurnLeftRight`
  (params (AxisValue :type "Float (single-precision)"))
  ;[1 1 1] Turn Left and Right
  (`self.AddControllerPitchInput` AxisValue))

(event `InputAxis|MoveLeftRight`
  (params (AxisValue :type "Float (single-precision)"))
  ;[1 1 1] Player Movement
  (`self.AddMovementInput` (`KismetMathLibrary.GetRightVector` (`KismetMathLibrary.MakeRotator` 0.0 0.0 (.yaw (`self.GetControlRotation`)))) AxisValue))

(event `InputAxis|MoveForwardsBackwards`
  (params (AxisValue :type "Float (single-precision)"))
  ;[1 1 1] Player Movement
  (`self.AddMovementInput` (`KismetMathLibrary.GetForwardVector` (`KismetMathLibrary.MakeRotator` 0.0 0.0 (.yaw (`self.GetControlRotation`)))) AxisValue))

(fn `UserConstructionScript`)